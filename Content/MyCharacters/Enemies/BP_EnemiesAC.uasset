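; AI controller for enemies that starts the BT_EnemiesAI behavior tree on BeginPlay.
; AI Perception updates feed a TargetActor name to the Blackboard through SetObjectParameter interface messages, rather than Set Value as Object.
; A successful sight stimulus passes the sensed actor.
; Lost sight or any non-sight stimulus sends the same message with no actor.
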(event `self.ReceiveBeginPlay`
  (`self.RunBehaviorTree` "/Game/MyCharacters/Enemies/BT_EnemiesAI.BT_EnemiesAI"))

(event `self.AIPerception.OnTargetPerceptionUpdated`
  (params (Actor :type "Actor Object Reference") (Stimulus :type "AIStimulus Structure"))
  (bind _returnvalue (`AIBlueprintHelperLibrary.GetBlackboard` null))
  (bind _returnvalue_2 (`AIPerceptionSystem.GetSenseClassForStimulus` Stimulus))
  (if (== _returnvalue_2 "/Script/AIModule.AISense_Sight")
    (if (`.bSuccessfullySensed` (break `AIStimulus` Stimulus))
      (message `AudioParameterControllerInterface.SetObjectParameter` _returnvalue "TargetActor" Actor)
      (else
        (message `AudioParameterControllerInterface.SetObjectParameter` _returnvalue "TargetActor" null :!label _label)))
    (else
      (goto _label))))

(fn `UserConstructionScript`)